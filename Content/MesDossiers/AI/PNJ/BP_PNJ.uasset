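; Quest-giver NPC that reacts when its PawnSensing component sees the player, driving its AI blackboard and dialogue.
; A retriggerable delay keeps the SeePlayer flag set during sighting, so quest logic runs only on each new sighting.
; It checks Initialiseur's quests to pick offer, unfinished or finished dialogue through the GameMode, using a gate for the finished case.
; Offering saves the first-meeting flag to the GameInstance, adds attached quests and can complete QuestToValidate.
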(event OnSeePawn(PawnSensing)
  (params (Pawn :type Pawn%20Object%20Reference))
  (bind _questattached (Variables|Default|GetQuestAttached))
  (bind _questattached_2 (Variables|Default|GetQuestAttached))
  (bind _questtovalidate (Variables|Default|GetQuestToValidate))
  (bind _initialiseur (Variables|Default|GetInitialiseur))
  (bind _initialiseur_2 (Variables|Default|GetInitialiseur))
  (bind _initialiseur_3 (Variables|Default|GetInitialiseur))
  (bind _quests (Variables|/Game/MesDossiers/Maps/BP_InitMap.BP_InitMap_C|GetQuests _initialiseur))
  (bind _quests_2 (Variables|/Game/MesDossiers/Maps/BP_InitMap.BP_InitMap_C|GetQuests _initialiseur_2))
  (Utilities|Casting|CastToBP_FirstPersonCharacter Pawn)
  (if (Variables|Default|GetTempBoolSeePlayer)
    (Variables|Default|SetTempBoolSeePlayer true :!label _label)
    (bind _asaic_pnj (Utilities|Casting|CastToAIC_PNJ (Pawn|GetController)))
    (AI|Components|Blackboard|SetValueasObject (AI|GetBlackboard _asaic_pnj) (Utilities|Name|MakeLiteralName "Player") (Variables|Default|GetPlayer))
    (AI|Components|Blackboard|SetValueasBool (AI|GetBlackboard _asaic_pnj) (Utilities|Name|MakeLiteralName "SeePlayer") (Variables|Default|GetTempBoolSeePlayer))
    (Utilities|FlowControl|RetriggerableDelay 0.2)
    (Variables|Default|SetTempBoolSeePlayer false)
    (AI|Components|Blackboard|SetValueasBool (AI|GetBlackboard _asaic_pnj) (Utilities|Name|MakeLiteralName "SeePlayer") (Variables|Default|GetTempBoolSeePlayer))
    (else
      (Utilities|FlowControl|Sequence
        (:then_0
          (goto _label))
        (:then_1
          (Variables|Default|SetTempBool false)
          (bind _index (Utilities|FlowControl|ForLoopwithBreak 0 (- (Utilities|Array|Length _quests) 1))
            (:LoopBody
              (if (== (Utilities|GetClass (Utilities|Array|Get(acopy) _quests _index)) (Utilities|Array|Get(acopy) (Variables|Default|GetQuestAttached)))
                (Variables|Default|SetTempBool true)))
            (:Completed
              (if (Variables|Default|GetTempBool)
                (Utilities|FlowControl|Sequence
                  (:then_0
                    (bind _index_2 (Utilities|FlowControl|ForLoopwithBreak 0 (- (Utilities|Array|Length _quests_2) 1) :!label _label_2)
                      (:LoopBody
                        (bind _index_3 (Utilities|FlowControl|ForLoopwithBreak 0 (- (Utilities|Array|Length _questattached_2) 1) :!label _label_3)
                          (:LoopBody
                            (if (== (Utilities|GetClass (Utilities|Array|Get(acopy) _quests_2 _index_2)) (Utilities|Array|Get(acopy) _questattached_2 _index_3))
                              (if (not (Variables|/Game/MesDossiers/Quest/Quest/BP_Quest.BP_Quest_C|GetCompleted (Utilities|Array|Get(acopy) _quests_2 _index_2)))
                                (Utilities|FlowControl|Sequence
                                  (:then_0
                                    (goto _label_4 Close))
                                  (:then_1
                                    (goto _label_2 Break))
                                  (:then_2
                                    (goto _label_3 Break))
                                  (:then_3
                                    (bind _asbp_game_mode (Utilities|Casting|CastToBP_GameMode (Game|GetGameMode)))
                                    (Default|PlayDialogue _asbp_game_mode (Variables|Default|GetDialoguesPasFini)))))))))
                      (:Completed
                        (Utilities|FlowControl|Gate false :!label _label_4
                          (:Exit
                            (bind _asbp_game_mode_2 (Utilities|Casting|CastToBP_GameMode (Game|GetGameMode)))
                            (Default|PlayDialogue _asbp_game_mode_2 (Variables|Default|GetDialoguesFini)))))))
                  (:then_1
                    (goto _label_4 Open)))
                (else
                  (bind _output_get (Variables|Default|SetFirstTime false))
                  (Variables|/Game/MesDossiers/GI_GameInstance.GI_GameInstance_C|SetPNJ1_FirstTime (Variables|Default|GetAs%20GI%20Game%20Instance) _output_get)
                  (bind _asbp_game_mode_3 (Utilities|Casting|CastToBP_GameMode (Game|GetGameMode)))
                  (Default|PlayDialogue _asbp_game_mode_3 (Variables|Default|GetDialoguesQuete) self)
                  (if (Utilities|IsValidClass (Utilities|Array|Get(acopy) (Variables|Default|GetQuestAttached)))
                    (for _index_4 (range 0 (- (Utilities|Array|Length _questattached) 1))
                      (Default|AddQuesttoGI _initialiseur_3 (Utilities|Array|Get(acopy) _questattached _index_4))
                      (if (Utilities|IsValidClass _questtovalidate)
                        (Default|SetQuestDone _initialiseur_3 _questtovalidate)))))))))))))

(event EventBeginPlay
  (bind _asbp_first_person_character (Utilities|Casting|CastToBP_FirstPersonCharacter (Game|GetPlayerCharacter 0)))
  (Variables|Default|SetPlayer _asbp_first_person_character)
  (bind _asgi_game_instance (Utilities|Casting|CastToGI_GameInstance (Game|GetGameInstance)))
  (bind _output_get (Variables|Default|SetAs%20GI%20Game%20Instance _asgi_game_instance))
  (Variables|Default|SetFirstTime (Variables|/Game/MesDossiers/GI_GameInstance.GI_GameInstance_C|GetPNJ1_FirstTime _output_get)))

(fn ConstructionScript)