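; BP_EnnemiParent is a parent enemy that dances in place and is killed when interacted with.
; From BeginPlay, it plays a random animation from Anims, waits a random few seconds, then repeats indefinitely.
; InteractItem searches the Initialiseur's quests for BP_QuestKillEnnemis, increments it, bumps the GameInstance's Map 2 dead-enemy count and destroys the actor.
; Destruction happens only inside that quest match, so without that quest the enemy remains.
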(event Custom|ChangeDance
  (bind _anims (Variables|Default|GetAnims))
  (bind _output_get (Variables|Default|SetMontagePlaying (Utilities|Array|Get(acopy) _anims (Math|Random|RandomIntegerinRange 0 (- (Utilities|Array|Length _anims) 1)))))
  (Components|Animation|PlayAnimation (Variables|Character|GetMesh) _output_get false)
  (Utilities|FlowControl|Delay (Math|Random|RandomFloatinRange 7.0 11.0))
  (if true
    (CallFunction|ChangeDance)))

(event EventInteractItem
  (for _array_element (Variables|/Game/MesDossiers/Maps/BP_InitMap.BP_InitMap_C|GetQuests (Variables|Default|GetInitialiseur))
    (if (== (Utilities|GetClass _array_element) "/Game/MesDossiers/Quest/Quest/BP_QuestKillEnnemis.BP_QuestKillEnnemis_C")
      (bind _asbp_quest_kill_ennemis (Utilities|Casting|CastToBP_QuestKillEnnemis _array_element))
      (Default|Incremente _asbp_quest_kill_ennemis)
      (bind _asgi_game_instance (Utilities|Casting|CastToGI_GameInstance (Game|GetGameInstance)))
      (Variables|/Game/MesDossiers/GI_GameInstance.GI_GameInstance_C|SetEnnemiDeadMap2 _asgi_game_instance (+ (Variables|/Game/MesDossiers/GI_GameInstance.GI_GameInstance_C|GetEnnemiDeadMap2 _asgi_game_instance) 1))
      (Actor|DestroyActor))))

(event EventBeginPlay
  (CallFunction|ChangeDance))

(fn ConstructionScript)