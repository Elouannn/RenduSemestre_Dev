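; BP_ExitLevel is a level exit trigger that moves the player on to the NextLevel map.
; When BP_FirstPersonCharacter overlaps its Box, a DoOnce passes the Quests of Initialiseur to GI_GameInstance through RegisterQuest, then opens the level after a short delay.
; BeginPlay caches the game instance, though the overlap casts it again, and CheckAnyQuest is a stub that always returns false.
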(event OnComponentBeginOverlap(Box)
  (params (OverlappedComponent :type Primitive%20Component%20Object%20Reference) (OtherActor :type Actor%20Object%20Reference) (OtherComp :type Primitive%20Component%20Object%20Reference) (OtherBodyIndex :type Integer) (bFromSweep :type Boolean) (SweepResult :type Hit%20Result%20Structure%20%28by%20ref%29))
  (Utilities|Casting|CastToBP_FirstPersonCharacter OtherActor)
  (Utilities|FlowControl|DoOnce false
    (:Completed
      (bind _asgi_game_instance (Utilities|Casting|CastToGI_GameInstance (Game|GetGameInstance)))
      (Default|RegisterQuest _asgi_game_instance (Variables|/Game/MesDossiers/Maps/BP_InitMap.BP_InitMap_C|GetQuests (Variables|Default|GetInitialiseur)))
      (Utilities|FlowControl|Delay 0.2)
      (Game|OpenLevel(byName) (Variables|Default|GetNextLevel)))))

(event EventBeginPlay
  (bind _asgi_game_instance (Utilities|Casting|CastToGI_GameInstance (Game|GetGameInstance)))
  (Variables|Default|SetGameInstance _asgi_game_instance))

(event Collision|EventActorBeginOverlap
  (params (OtherActor :type Actor%20Object%20Reference)))

(event EventTick
  (params (DeltaSeconds :type Float%20%28single-precision%29)))

(fn ConstructionScript)

(fn CheckAnyQuest
  (return false))