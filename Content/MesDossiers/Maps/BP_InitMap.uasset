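; BP_InitMap is a map initializer actor that sets up the level exit and manages quests for the current map.
; On BeginPlay it spawns BP_ExitLevel at the FakeExit placeholder, copies its NextLevel, and registers with GI_GameInstance.
; It binds player events, forwarding new quests to the game instance and validating requested quest classes against its Quests array.
; Completing a quest refreshes the WB_Quest widget, and validation results return to the player.
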(event Custom|QuestUI
  (Utilities|IsValid (Variables|Default|GetWB_Quete)
    (:Is%20Valid
      _)
    (:Is%20Not%20Valid
      (bind _returnvalue (UserInterface|CreateWidget "/Game/MesDossiers/UI/WB_Quest.WB_Quest_C" (Game|GetPlayerController 0)))
      (bind _output_get (Variables|Default|SetWB_Quete _returnvalue))
      (UserInterface|Viewport|AddtoViewport _output_get 0)))
  (Default|MajText (Variables|Default|GetWB_Quete) (Variables|Default|GetQuests)))

(event Custom|SetQuestDone
  (params (Quest%20to%20validate :type BP%20Quest%20Class%20Reference))
  (bind _quests (Variables|Default|GetQuests))
  (bind _index (Utilities|FlowControl|ForLoopwithBreak 0 (- (Utilities|Array|Length _quests) 1) :!label _label)
    (:LoopBody
      (if (== (Utilities|GetClass (Utilities|Array|Get(acopy) _quests _index)) Quest%20to%20validate)
        (Utilities|FlowControl|Sequence
          (:then_0
            (goto _label Break))
          (:then_1
            (Variables|/Game/MesDossiers/Quest/Quest/BP_Quest.BP_Quest_C|SetCompleted (Utilities|Array|Get(acopy) _quests _index) true)))))
    (:Completed
      (CallFunction|QuestUI))))

(event Custom|AddQuestToGI
  (params (QuestToAdd :type BP%20Quest%20Class%20Reference))
  (Default|CreateQuest (Variables|Default|GetGameInstance) QuestToAdd))

(event Custom|ValidateQuestFromPlayer
  (bind _player (Variables|Default|GetPlayer))
  (bind _tempvarquest (Variables|/Game/FirstPerson/Blueprints/BP_FirstPersonCharacter.BP_FirstPersonCharacter_C|GetTempVarQuest _player))
  (Variables|Default|SetTempBool false)
  (for _index (range 0 (- (Utilities|Array|Length _tempvarquest) 1))
    (if (Utilities|IsValidClass (Utilities|Array|Get(acopy) _tempvarquest _index))
      (bind _array_element (Utilities|Array|ForEachLoopwithBreak (Variables|Default|GetQuests) :!label _label)
        (:LoopBody
          (if (== (Utilities|GetClass _array_element) (Utilities|Array|Get(acopy) _tempvarquest _index))
            (if (not (Variables|/Game/MesDossiers/Quest/Quest/BP_Quest.BP_Quest_C|GetCompleted _array_element))
              (CallFunction|SetQuestDone (Utilities|Array|Get(acopy) _tempvarquest _index))
              (Variables|Default|SetTempBool true)
              (goto _label Break)))))))
  (Default|QuestAccepted (Variables|Default|GetPlayer) (Variables|Default|GetTempBool)))

(event Custom|getQuestToAdd
  (for _array_element (Variables|/Game/FirstPerson/Blueprints/BP_FirstPersonCharacter.BP_FirstPersonCharacter_C|GetTempVarQuestToAdd (Variables|Default|GetPlayer))
    (CallFunction|AddQuesttoGI _array_element)))

(event EventBeginPlay
  (bind _fakeexit (Variables|Default|GetFakeExit))
  (bind _returnvalue (Game|SpawnActorfromClass "/Game/MesDossiers/Maps/BP_ExitLevel.BP_ExitLevel_C" (Transformation|GetActorTransform _fakeexit) "Undefined" "MultiplyWithRoot" 0 0))
  (bind _output_get (Variables|Default|SetExit _returnvalue))
  (Variables|/Game/MesDossiers/Maps/BP_ExitLevel.BP_ExitLevel_C|SetNextLevel _output_get (Variables|/Game/MesDossiers/Maps/BP_FakeExit.BP_FakeExit_C|GetNextLevel _fakeexit))
  (Variables|/Game/MesDossiers/Maps/BP_ExitLevel.BP_ExitLevel_C|SetInitialiseur _output_get self)
  (bind _asgi_game_instance (Utilities|Casting|CastToGI_GameInstance (Game|GetGameInstance)))
  (bind _output_get_2 (Variables|Default|SetGameInstance _asgi_game_instance))
  (Default|OpenNewMap _output_get_2 self)
  (bind _asbp_first_person_character (Utilities|Casting|CastToBP_FirstPersonCharacter (Game|GetPlayerCharacter 0)))
  (bind _output_get_3 (Variables|Default|SetPlayer _asbp_first_person_character))
  (EventDispatchers|BindEventtoTryValidateQuest _output_get_3 (delegate Custom|ValidateQuestFromPlayer))
  (EventDispatchers|BindEventtoAddQuestfromPlayer _output_get_3 (delegate Custom|getQuestToAdd)))

(fn ConstructionScript)