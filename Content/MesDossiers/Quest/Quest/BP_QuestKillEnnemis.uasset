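; Quest actor Blueprint for a kill-enemies objective, tracking a kill count against a target.
; Each Incremente event adds one to ActualInteger and compares it with TargetInteger.
; Once the target is reached, a DoOnce gate has Initialiseur mark this quest class as done through SetQuestDone, so completion is reported a single time.
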(event Custom|Incremente
  ;[1 1 1] Incrémentation du compteur de kill
  (bind _output_get (Variables|Default|SetActualInteger (+ (Variables|Default|GetActualInteger) 1)))
  (if (>= _output_get (Variables|Default|GetTargetInteger))
    (Utilities|FlowControl|DoOnce false
      (:Completed
        (Default|SetQuestDone (Variables|Default|GetInitialiseur) (Utilities|GetClass self))))))

(event EventBeginPlay
  (|CallParentFunction) ; This node is disabled and will not be called.\nDrag off pins to build functionality.
)

(event Collision|EventActorBeginOverlap
  (params (OtherActor :type Actor%20Object%20Reference))
  (|CallParentFunction OtherActor) ; This node is disabled and will not be called.\nDrag off pins to build functionality.
)

(event EventTick
  (params (DeltaSeconds :type Float%20%28single-precision%29))
  (|CallParentFunction DeltaSeconds) ; This node is disabled and will not be called.\nDrag off pins to build functionality.
)

(fn ConstructionScript
  (|CallParentFunction))