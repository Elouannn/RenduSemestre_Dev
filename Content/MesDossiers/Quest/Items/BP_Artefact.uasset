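; BP_Artefact is an interactable quest item that the player can pick up.
; InteractItem asks the Player to validate the item's QuestToValidate.
; When TryValidate reports success, it sets the Player's ObjectInHand to its own class, adds QuestAttached to the Player and destroys itself.
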(event EventBeginPlay
  (|CallParentFunction) ; This node is disabled and will not be called.\nDrag off pins to build functionality.
)

(event Collision|EventActorBeginOverlap
  (params (OtherActor :type Actor%20Object%20Reference))
  (|CallParentFunction OtherActor) ; This node is disabled and will not be called.\nDrag off pins to build functionality.
)

(event EventTick
  (params (DeltaSeconds :type Float%20%28single-precision%29))
  (|CallParentFunction DeltaSeconds) ; This node is disabled and will not be called.\nDrag off pins to build functionality.
)

(event EventInteractItem
  (Default|ValidateQuest (Variables|Default|GetPlayer) (Variables|Default|GetQuestToValidate)))

(event EventTryValidate
  (params (Success :type Boolean))
  (bind _player (Variables|Default|GetPlayer))
  (if Success
    (Variables|/Game/FirstPerson/Blueprints/BP_FirstPersonCharacter.BP_FirstPersonCharacter_C|SetObjectInHand _player (Utilities|GetClass self))
    (Default|AddQuest _player (Variables|Default|GetQuestAttached))
    (Actor|DestroyActor)))

(fn ConstructionScript
  (|CallParentFunction))