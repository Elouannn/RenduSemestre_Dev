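; BP_Slot is an interactable quest slot where the player places or retrieves a held artefact.
; InteractItem moves the item between StoredActor and the player's ObjectInHandTemp, toggling Artefact visibility, and asks the player to validate the quest on put-down.
; On success, TryValidate clears ObjectInHand, destroys linked actors, adds the next quest, and replaces the slot with a BP_ExitLevel spawned at ExitToCreate's location, inheriting its NextLevel.
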(event Custom|SpawnFinalExit
  (bind _exittocreate (Variables|Default|GetExitToCreate))
  (bind _returnvalue (Game|SpawnActorfromClass "/Game/MesDossiers/Maps/BP_ExitLevel.BP_ExitLevel_C" (Math|Transform|MakeTransform (Transformation|GetActorLocation _exittocreate) "0, 0, 0" "1.000000,1.000000,1.000000") "Undefined" "MultiplyWithRoot" 0 0))
  (Variables|/Game/MesDossiers/Maps/BP_ExitLevel.BP_ExitLevel_C|SetInitialiseur _returnvalue (Variables|Default|GetInitialiseur))
  (Variables|/Game/MesDossiers/Maps/BP_ExitLevel.BP_ExitLevel_C|SetNextLevel _returnvalue (Variables|/Game/MesDossiers/Maps/BP_FakeExit.BP_FakeExit_C|GetNextLevel _exittocreate))
  (Default|SetText _returnvalue)
  (Actor|DestroyActor))

(event EventBeginPlay)

(event EventInteractItem
  (bind _player (Variables|Default|GetPlayer))
  (bind _artefact (Variables|Default|GetArtefact))
  (if (Utilities|IsValidClass (Variables|/Game/FirstPerson/Blueprints/BP_FirstPersonCharacter.BP_FirstPersonCharacter_C|GetObjectInHand (Variables|Default|GetPlayer)))
    (if (Utilities|IsValidClass (Variables|Default|GetStoredActor))
      (if (Utilities|IsValidClass (Variables|/Game/FirstPerson/Blueprints/BP_FirstPersonCharacter.BP_FirstPersonCharacter_C|GetObjectInHandTemp _player))
        (Development|PrintString "Main pleine")
        (else
          (Variables|/Game/FirstPerson/Blueprints/BP_FirstPersonCharacter.BP_FirstPersonCharacter_C|SetObjectInHandTemp _player (Variables|Default|GetStoredActor))
          (Variables|Default|SetStoredActor 0)
          (Development|PrintString "PickUp")
          (Development|SetHiddeninGame _artefact true false)))
      (elif (Utilities|IsValidClass (Variables|/Game/FirstPerson/Blueprints/BP_FirstPersonCharacter.BP_FirstPersonCharacter_C|GetObjectInHandTemp _player))
        (Variables|Default|SetStoredActor (Variables|/Game/FirstPerson/Blueprints/BP_FirstPersonCharacter.BP_FirstPersonCharacter_C|GetObjectInHandTemp _player))
        (Variables|/Game/FirstPerson/Blueprints/BP_FirstPersonCharacter.BP_FirstPersonCharacter_C|SetObjectInHandTemp _player 0)
        (Development|PrintString "PutDown")
        (Development|SetHiddeninGame _artefact false false)
        (Default|ValidateQuest (Variables|Default|GetPlayer) (Variables|Default|GetQuestToValidate) self)
        (else
          (Development|PrintString "Main vide"))))))

(event EventTryValidate
  (params (Success :type Boolean))
  (bind _linkedactordestroy (Variables|Default|GetLinkedActorDestroy))
  (if Success
    (Variables|/Game/FirstPerson/Blueprints/BP_FirstPersonCharacter.BP_FirstPersonCharacter_C|SetObjectInHand (Variables|Default|GetPlayer) 0)
    (for _index (range 0 (- (Utilities|Array|Length _linkedactordestroy) 1))
      (Actor|DestroyActor (Utilities|Array|Get(acopy) _linkedactordestroy _index)))
    (Default|AddQuest (Variables|Default|GetPlayer) (Variables|Default|GetQuestToAdd))
    (CallFunction|SpawnFinalExit)))

(fn ConstructionScript)