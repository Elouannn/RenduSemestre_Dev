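; BP_GameMode is a Game Mode Blueprint that plays timed dialogue sequences on screen.
; PlayDialogue resets the line index, adds a new WB_Dialogue widget to the viewport and shows the first line immediately.
; A looping TimeToRead timer calls ChangeText to advance through the Dialogues array, then clears itself and removes the widget after the last line.
; The WhoIsSelf input is unused.
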(event Custom|PlayDialogue
  (params (Dialogues :type Array%20of%20Texts) (WhoIsSelf :type BP%20PNJ%20Object%20Reference))
  (Variables|Default|SetTempVarDialogue 0)
  (bind _returnvalue (UserInterface|CreateWidget "/Game/MesDossiers/UI/WB_Dialogue.WB_Dialogue_C" (Game|GetPlayerController 0)))
  (bind _output_get (Variables|Default|SetDialogueWidget _returnvalue))
  (UserInterface|Viewport|AddtoViewport _output_get 0)
  (CallFunction|ChangeText)
  (bind _returnvalue_2 (Utilities|Time|SetTimerbyEvent (delegate Custom|ChangeText) (Variables|Default|GetTimeToRead) true))
  (Variables|Default|SetSpawnTimer _returnvalue_2))

(event Custom|ChangeText
  (if (>= (Variables|Default|GetTempVarDialogue) (Utilities|Array|Length (stale Custom|PlayDialogue Dialogues)))
    (Utilities|Time|ClearandInvalidateTimerbyHandle (Variables|Default|GetSpawnTimer))
    (Widget|RemovefromParent (Variables|Default|GetDialogueWidget))
    (else
      (Variables|/Game/MesDossiers/UI/WB_Dialogue.WB_Dialogue_C|SetTextDialogue (Variables|Default|GetDialogueWidget) (Utilities|Array|Get(acopy) (stale Custom|PlayDialogue Dialogues) (Variables|Default|GetTempVarDialogue)))
      (Variables|Default|SetTempVarDialogue (+ (Variables|Default|GetTempVarDialogue) 1)))))

(event EventBeginPlay)

(fn ConstructionScript)